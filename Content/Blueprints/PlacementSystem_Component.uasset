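; Actor component for BP_ThirdPersonCharacter that places BP_Cube actors on surfaces the player aims at.
; While left mouse is held, Tick line-traces from the follow camera, storing the impact point if the hit component carries the placeable tag.
; With the button up, Tick spawns a cube at that point.
; The placement flag is not cleared after spawning, so spawning repeats every tick.
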(event `self.ReceiveBeginPlay`
  (bind _asbp_third_person_character (cast `/Game/ThirdPerson/Blueprints/BP_ThirdPersonCharacter` (`self.GetOwner`)))
  (set `self.Follow Camera` (`/Game/ThirdPerson/Blueprints/BP_ThirdPersonCharacter.FollowCamera` _asbp_third_person_character)))

(event `self.ReceiveTick`
  (params (DeltaSeconds :type "Float (single-precision)"))
  (if (`PlayerController.IsInputKeyDown` (`GameplayStatics.GetPlayerController` 0) "LeftMouseButton")
    (bind (_ishittingground _hitposition) (`self.IisHittingGround`))
    (bind _output_get (set `self.Can Place Objects` _ishittingground))
    (if _output_get
      (set `self.Hit Position` _hitposition))
    (elif (`self.Can Place Objects`)
      (`self.PlaceObject` (`self.Hit Position`)))))

(fn `IisHittingGround`
  (returns (isHittingGround :type Boolean) (hitPosition :type "Vector Structure"))
  (bind _follow_camera (`self.Follow Camera`))
  (bind _returnvalue (`SceneComponent.K2_GetComponentLocation` _follow_camera))
  (bind (_bblockinghit _binitialoverlap _time _distance _location _impactpoint _normal _impactnormal _physmat _hitactor _hitcomponent) (`GameplayStatics.BreakHitResult` (`self.hitInfo`)))
  (bind (_outhit _returnvalue_2) (`KismetSystemLibrary.LineTraceSingle` _returnvalue (+ _returnvalue (* (`SceneComponent.GetForwardVector` _follow_camera) (`self.RayDistance`))) "TraceTypeQuery1"))
  (set `self.hitInfo` _outhit)
  (if _returnvalue_2
    (if (`self.ComponentHasTag` _hitcomponent (`self.PlaceableObjectsTag`))
      (return true _impactpoint))
    (else
      (return false (0.0 0.0 0.0)))))

(fn `PlaceObject`
  (params (LocationToPlace :type "Vector Structure"))
  (`|SpawnActorFromClass` "/Game/Blueprints/BP_Cube.BP_Cube_C" (`KismetMathLibrary.Conv_VectorToTransform` LocationToPlace) "Undefined" "MultiplyWithRoot" null null))